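; Behavior tree task that asks a question with selectable responses in the dialogue UI.
; On AI execute, it gets the dialogue box widget from a blackboard key and sets its text to the question.
; It then adds a response list widget to the box and fills it with one response widget per answer text.
; The graph shows no finish call or handling of the chosen response.
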(event EventReceiveExecuteAI
  (params (OwnerController :type AI%20Controller%20Object%20Reference) (ControlledPawn :type Pawn%20Object%20Reference))
  (bind _aswb_dialouge_box (Utilities|Casting|CastToWB_DialougeBox (Class|BTFunctionLibrary|GetBlackboardValueasObject (Variables|Default|GetBB_DialogueUI))))
  (bind _output_get (Variables|Default|SetDialougeBoxUI _aswb_dialouge_box))
  (Variables|/Game/Blueprint/Interaction_Interfaces/WB_DialougeBox.WB_DialougeBox_C|SetDialougeText _output_get (Variables|Default|GetQuestion))
  (CallFunction|PrepareResponses))

(fn PrepareResponses
  (bind _returnvalue (UserInterface|CreateWidget "/Game/Blueprint/Interaction_Interfaces/WB_ResponseListUI.WB_ResponseListUI_C"))
  (bind _output_get (Variables|Default|SetResponseListUI _returnvalue))
  (Class|Overlay|AddChildtoOverlay (Variables|/Game/Blueprint/Interaction_Interfaces/WB_DialougeBox.WB_DialougeBox_C|GetResponseListPanel (Variables|Default|GetDialougeBoxUI)) _output_get)
  (for _array_element (Variables|Default|GetResponses)
    (bind _returnvalue_2 (UserInterface|CreateWidget "/Game/Blueprint/Interaction_Interfaces/WB_ResponseUI.WB_ResponseUI_C" 0 _array_element))
    (Class|VerticalBox|AddChildtoVerticalBox (Variables|/Game/Blueprint/Interaction_Interfaces/WB_ResponseListUI.WB_ResponseListUI_C|GetResponseList (Variables|Default|GetResponseListUI)) _returnvalue_2)))