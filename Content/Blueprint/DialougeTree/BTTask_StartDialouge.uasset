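; Behavior tree task that begins a dialogue in the dialogue tree system.
; It makes the dialogue box from the game mode's InteractUI visible and stores that widget in a blackboard key, presumably for other tasks to use.
; It then disables the player character's input, hides the mouse cursor and finishes successfully.
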(event EventReceiveExecuteAI
  (params (OwnerController :type AI%20Controller%20Object%20Reference) (ControlledPawn :type Pawn%20Object%20Reference))
  (bind _returnvalue (Game|GetPlayerController 0))
  (bind _asthird_person_game_mode (Utilities|Casting|CastToThirdPersonGameMode (Game|GetGameMode)))
  (Widget|SetVisibility (Variables|/Game/Blueprint/Interaction_Interfaces/WB_InteractUI.WB_InteractUI_C|GetWB_DialougeBox (Variables|/Game/ThirdPersonBP/Blueprints/ThirdPersonGameMode.ThirdPersonGameMode_C|GetInteractUI _asthird_person_game_mode)) "Visible")
  (Class|BTFunctionLibrary|SetBlackboardValueasObject (Variables|Default|GetBB_DialogueUI) (Variables|/Game/Blueprint/Interaction_Interfaces/WB_InteractUI.WB_InteractUI_C|GetWB_DialougeBox (Variables|/Game/ThirdPersonBP/Blueprints/ThirdPersonGameMode.ThirdPersonGameMode_C|GetInteractUI _asthird_person_game_mode)))
  (Input|DisableInput (Game|GetPlayerCharacter 0) _returnvalue)
  (Variables|/Script/Engine.PlayerController|SetbShowMouseCursor _returnvalue false)
  (AI|BehaviorTree|FinishExecute true))